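; BP_Dropper is an actor that wanders autonomously, avoiding obstacles and dropping spheres as it goes.
; Its behavior is composed of instruction objects built in the Construction Script and configured on BeginPlay.
; Each Tick feeds delta time to a Wait instruction, which gates every step.
; When it passes, a collision check selects either a random-angle rotation or a forward move, then DropSphere runs.
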(event `self.ReceiveBeginPlay`
  (bind _inst_moveforward (`self.Inst_MoveForward`))
  (bind _inst_iscolliding (`self.Inst_IsColliding`))
  (bind _inst_calculaterandomangle (`self.Inst_CalculateRandomAngle`))
  (bind _inst_wait (`self.Inst_Wait`))
  (bind _inst_dropsphere (`self.Inst_DropSphere`))
  (`RobotInstruction.BeginPlayObject` _inst_moveforward)
  (set `MoveForward.mMoveDistance` 10.0 _inst_moveforward)
  (`RobotInstruction.BeginPlayObject` _inst_iscolliding)
  (set `IsColliding.mObstacleDistance` 150.0 _inst_iscolliding)
  (`RobotInstruction.BeginPlayObject` (`self.Inst_Rotate`))
  (set `CalculateRandomAngle.mMinAngle` 5.0 _inst_calculaterandomangle)
  (set `CalculateRandomAngle.mMaxAngle` 25.0 _inst_calculaterandomangle)
  (`RobotInstruction.BeginPlayObject` _inst_wait)
  (set `Wait.mTimeToWait` 1.0 _inst_wait)
  (`RobotInstruction.BeginPlayObject` _inst_dropsphere)
  (set `DropSphere.mSphereDistance` -100.0 _inst_dropsphere))

(event `self.ReceiveTick`
  (params (DeltaSeconds :type "Float (single-precision)"))
  (bind _inst_rotate (`self.Inst_Rotate`))
  (bind _inst_wait (`self.Inst_Wait`))
  (bind _inst_calculaterandomangle (`self.Inst_CalculateRandomAngle`))
  (set `Wait.mDeltaTime` DeltaSeconds _inst_wait)
  (bind _returnvalue (`RobotInstruction.ExecuteInstruction` _inst_wait self))
  (if _returnvalue
    (bind _returnvalue_2 (`RobotInstruction.ExecuteInstruction` (`self.Inst_IsColliding`) self))
    (if _returnvalue_2
      (`RobotInstruction.ExecuteInstruction` _inst_calculaterandomangle self)
      (bind _returnvalue_3 (`CalculateRandomAngle.GetRandomAngle` _inst_calculaterandomangle))
      (bind _returnvalue_4 (`CalculateRandomAngle.GetRandomDirection` _inst_calculaterandomangle))
      (set `Rotate.mRotationAngle` _returnvalue_3 _inst_rotate)
      (set `Rotate.mRotationDirection` _returnvalue_4 _inst_rotate)
      (`RobotInstruction.ExecuteInstruction` _inst_rotate self)
      (else
        (`RobotInstruction.ExecuteInstruction` (`self.Inst_MoveForward`) self)))
    (`RobotInstruction.ExecuteInstruction` (`self.Inst_DropSphere`) self)))

(fn `UserConstructionScript`
  (bind _returnvalue (`|GenericCreateObject` "/Script/AIREngineerTest.MoveForward" self))
  (set `self.Inst_MoveForward` _returnvalue)
  (bind _returnvalue_2 (`|GenericCreateObject` "/Script/AIREngineerTest.IsColliding" self))
  (set `self.Inst_IsColliding` _returnvalue_2)
  (bind _returnvalue_3 (`|GenericCreateObject` "/Script/AIREngineerTest.Rotate" self))
  (set `self.Inst_Rotate` _returnvalue_3)
  (bind _returnvalue_4 (`|GenericCreateObject` "/Script/AIREngineerTest.CalculateRandomAngle" self))
  (set `self.Inst_CalculateRandomAngle` _returnvalue_4)
  (bind _returnvalue_5 (`|GenericCreateObject` "/Script/AIREngineerTest.Wait" self))
  (set `self.Inst_Wait` _returnvalue_5)
  (bind _returnvalue_6 (`|GenericCreateObject` "/Script/AIREngineerTest.DropSphere" self))
  (set `self.Inst_DropSphere` _returnvalue_6))